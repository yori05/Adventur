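; Character that can be targeted and interacted with, showing markers for targeting state and toggling ragdoll on interact.
; BeginPlay binds to TargetableComponent events, which show or hide a Sphere while focused and a Cube while locked.
; Each interact flip-flops between pelvis-down ragdoll with particles active and restoring the mesh's collision, attachment to the capsule and relative transform.
; Capsule collision changes are present but unconnected.
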(event `self.ReceiveBeginPlay`
  (bind _targetablecomponent (`self.TargetableComponent`))
  (add `TargetableComponent.OnTargetBeginFocus` _targetablecomponent (delegate `OnBeginFocused`))
  (add `TargetableComponent.OnTargetEndFocus` _targetablecomponent (delegate `OnEndFocused`))
  (add `TargetableComponent.OnTargetBeginLocked` _targetablecomponent (delegate `OnBeginLocked`))
  (add `TargetableComponent.OnTargetEndLocked` _targetablecomponent (delegate `OnEndLocked`)))

(event `OnBeginFocused`
  (`SceneComponent.SetVisibility` (`self.Sphere`) true false))

(event `OnBeginLocked`
  (`SceneComponent.SetVisibility` (`self.Cube`) true false))

(event `OnEndFocused`
  (`SceneComponent.SetVisibility` (`self.Sphere`) false false))

(event `OnEndLocked`
  (`SceneComponent.SetVisibility` (`self.Cube`) false false))

(event `InteractibleInterface.OnBeginInteract`
  (params (Caller :type "Actor Object Reference"))
  (bind _particlesystem (`self.ParticleSystem`))
  (bind _mesh (`self.Mesh`))
  (bind _mesh_2 (`self.Mesh`))
  (`/Engine/EditorBlueprintResources/StandardMacros.FlipFlop`
    (:`A`
      (`ActorComponent.SetActive` _particlesystem true false)
      (`SkeletalMeshComponent.SetAllBodiesBelowSimulatePhysics` _mesh "pelvis" true true)
      (`SkeletalMeshComponent.SetAllBodiesBelowPhysicsBlendWeight` _mesh "pelvis" 1.0 false true)
      (`PrimitiveComponent.SetCollisionProfileName` _mesh_2 "Ragdoll" true))
    (:`B`
      (`ActorComponent.SetActive` _particlesystem false false)
      (`SkeletalMeshComponent.SetAllBodiesBelowSimulatePhysics` _mesh "pelvis" false true)
      (`SkeletalMeshComponent.SetAllBodiesBelowPhysicsBlendWeight` _mesh "pelvis" 0.0 false true)
      (`PrimitiveComponent.SetCollisionProfileName` _mesh_2 "CharacterMesh" true)
      (`SceneComponent.K2_AttachToComponent` _mesh_2 (`self.CapsuleComponent`) "None" "KeepRelative" "KeepRelative" "KeepRelative" true)
      (`SceneComponent.K2_SetRelativeLocationAndRotation` _mesh_2 (0.0 0.0 -90.0) (struct :`Yaw` -90.0) false false))))

(event `InteractibleInterface.OnStopInteract`
  (params (Caller :type "Actor Object Reference")))

(event `InteractibleInterface.BeginFocus`)

(event `InteractibleInterface.StopFocus`)

(fn `UserConstructionScript`)