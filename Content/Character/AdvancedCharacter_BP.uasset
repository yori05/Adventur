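; AdvancedCharacter_BP is a character Blueprint that lets the player interact with targeted objects.
; On Interact input press, it asks its LockerComponent for the current target and validates that target and its owner.
; If the owner implements InteractibleInterface, it sends OnBeginInteract to that actor, passing itself as the interactor.
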(event `InputAction|Interact`
  (params (Key :type "Key Structure"))
  (bind _lockercomponent (`self.LockerComponent`))
  (:`Pressed`
    (`/Engine/EditorBlueprintResources/StandardMacros.IsValid` _lockercomponent
      (:`Is Valid`
        (bind _returnvalue (`LockerComponent.HasATarget` _lockercomponent))
        (if _returnvalue
          (bind _returnvalue_2 (`LockerComponent.GetCurrentTarget` _lockercomponent))
          (`/Engine/EditorBlueprintResources/StandardMacros.IsValid` _returnvalue_2
            (:`Is Valid`
              (bind _returnvalue_3 (`ActorComponent.GetOwner` _returnvalue_2))
              (`/Engine/EditorBlueprintResources/StandardMacros.IsValid` _returnvalue_3
                (:`Is Valid`
                  (if (`KismetSystemLibrary.DoesImplementInterface` _returnvalue_3 "/Script/Adventur.InteractibleInterface")
                    (message `InteractibleInterface.OnBeginInteract` _returnvalue_3 self)))))))))))

(fn `UserConstructionScript`)